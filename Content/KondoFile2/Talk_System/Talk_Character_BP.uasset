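; Talkable character Blueprint that shows when the player is in conversation range and turns to face them.
; A box trigger plays and reverses the Size timeline on player overlap, which scales the widget's draw size.
; CanTalk checks that the player is inside the box, then starts the Rotation timeline to blend the actor's rotation toward the player and returns the overlap result.
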(event `self.ReceiveBeginPlay`)

(event `self.Box.OnComponentBeginOverlap`
  (params (OverlappedComponent :type "PrimitiveComponent Object Reference") (OtherActor :type "Actor Object Reference") (OtherComp :type "PrimitiveComponent Object Reference") (OtherBodyIndex :type Integer) (bFromSweep :type Boolean) (SweepResult :type "HitResult Structure (by ref)"))
  (if (== OtherActor (`GameplayStatics.GetPlayerCharacter` 0))
    (`TimelineComponent.Play` (`self.Size`))))

(event `self.Box.OnComponentEndOverlap`
  (params (OverlappedComponent :type "PrimitiveComponent Object Reference") (OtherActor :type "Actor Object Reference") (OtherComp :type "PrimitiveComponent Object Reference") (OtherBodyIndex :type Integer))
  (if (== OtherActor (`GameplayStatics.GetPlayerCharacter` 0))
    (`TimelineComponent.Reverse` (`self.Size`))))

(fn `CanTalk?`
  (returns (`CanTalk?` :type Boolean))
  (bind _returnvalue (`PrimitiveComponent.IsOverlappingActor` (`self.Box`) (`GameplayStatics.GetPlayerCharacter` 0)))
  (if _returnvalue
    (`TimelineComponent.PlayFromStart` (`self.Rotation`))
    (return _returnvalue)))

(fn `UserConstructionScript`)