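; BP_interactOBJbase is a base interactable object actor that runs a temporary item-get interaction with the player.
; The BPIGetItemStart event enables player input on the actor and opens a Gate on Tick, which currently only prints a debug string.
; Pressing E disables input, sends BPIGetItemEndMessage to the player controller and closes the Gate.
; BeginPlay caches the root's relative location, which is not used elsewhere here.
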(event `self.ReceiveBeginPlay`
  (set `self.DefoultPosition` (`SceneComponent.RelativeLocation` (`self.DefaultSceneRoot`))))

(event `self.ReceiveTick`
  (params (DeltaSeconds :type "Float (single-precision)"))
  (`/Engine/EditorBlueprintResources/StandardMacros.Gate` true :!label _label
    (:`Exit`
      (`KismetSystemLibrary.PrintString` "Hello"))))

(event `/Game/kuwano_folder/BP/BPI_HitNotify.BPI_GetItemStart`
  (`self.EnableInput` (`GameplayStatics.GetPlayerController` 0))
  (goto _label :!via `Open`))

(event `Key|E`
  (params (Key :type "Key Structure"))
  (:`Pressed`
    (`self.DisableInput` (`GameplayStatics.GetPlayerController` 0))
    (message `/Game/kuwano_folder/BP/BPI_HitNotify.BPI_GetItemEnd` (`GameplayStatics.GetPlayerController` 0))
    (goto _label :!via `Close`)))

(fn `UserConstructionScript`)