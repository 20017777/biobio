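; BP_ItemHeal is a pickup item actor, named as a healing item, that carries its own item info struct.
; On BeginPlay it rebuilds that struct, keeping the existing fields but filling in its own class and current actor scale.
; GetItemInfo returns the struct, and ActionPIck destroys the actor.
; HP_count_loss is an empty event, so no healing logic runs here.
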(event `self.ReceiveBeginPlay`
  (bind (_itemname _itemcount _itemexplanation _en_itemcategory _itemimage) (break `/Game/kuwano_folder/BP/ST_ItemInfo` (`self.ST Item Heal Info`)))
  (set `self.ST Item Heal Info` (make `/Game/kuwano_folder/BP/ST_ItemInfo` _itemname _itemcount _itemexplanation _en_itemcategory _itemimage (`GameplayStatics.GetObjectClass` self) (`self.GetActorScale3D`))))

(event `HP_count_loss`)

(event `/Game/kuwano_folder/BP/BPI_PickItem.ActionPIck`
  (`self.K2_DestroyActor`))

(fn `GetItemInfo`
  (returns (ST_ItemInfo :type "/Game/kuwano_folder/BP/ST_ItemInfo Structure"))
  (return (`self.ST Item Heal Info`)))

(fn `UserConstructionScript`)