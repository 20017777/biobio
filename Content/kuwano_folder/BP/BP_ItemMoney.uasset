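; BP_ItemMoney is a money item actor that can be picked up and exposes its item data.
; On BeginPlay it rebuilds its item info struct, keeping the set name, count, explanation, category and image while filling in its own class and actor scale.
; GetItemInfo returns that struct, and the ActionPIck event simply destroys the actor.
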(event `self.ReceiveBeginPlay`
  (bind (_itemname _itemcount _itemexplanation _en_itemcategory _itemimage) (break `/Game/kuwano_folder/BP/ST_ItemInfo` (`self.ST Item Money Info`)))
  (set `self.ST Item Money Info` (make `/Game/kuwano_folder/BP/ST_ItemInfo` _itemname _itemcount _itemexplanation _en_itemcategory _itemimage (`GameplayStatics.GetObjectClass` self) (`self.GetActorScale3D`))))

(event `/Game/kuwano_folder/BP/BPI_PickItem.ActionPIck`
  (`self.K2_DestroyActor`))

(fn `GetItemInfo`
  (returns (ST_ItemInfo :type "/Game/kuwano_folder/BP/ST_ItemInfo Structure"))
  (return (`self.ST Item Money Info`)))

(fn `UserConstructionScript`
  (`parent.UserConstructionScript`))