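; BP_enemy is a melee enemy, animated with a zombie attack montage, with health and a floating HP bar.
; Damage lowers HP, and death rolls chained random checks to possibly drop an ammo, heal or money item before destroying the actor.
; Tick feeds HP to the widget, turns it toward the camera and shows it only when the player is near.
; A toggleable Box hitbox damages the player on overlap, throttled by a short DoOnce delay.
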(event `self.ReceiveAnyDamage`
  (params (Damage :type "Float (single-precision)") (DamageType :type "DamageType Object Reference") (InstigatedBy :type "Controller Object Reference") (DamageCauser :type "Actor Object Reference"))
  (bind _output_get (set `self.HP` (- (`self.HP`) Damage)))
  (if (<= _output_get 0.0)
    (if (> (`KismetMathLibrary.RandomInteger` 10) 6)
      (`|SpawnActorFromClass` "/Game/kuwano_folder/BP/BP_ItemAmmo.BP_ItemAmmo_C" (`KismetMathLibrary.MakeTransform` (`self.K2_GetActorLocation`) (`KismetMathLibrary.RandomRotator` false)) "Undefined" "OverrideRootScale" null null)
      (elif (> (`KismetMathLibrary.RandomInteger` 7) 3)
        (`|SpawnActorFromClass` "/Game/kuwano_folder/BP/BP_ItemHeal.BP_ItemHeal_C" (`KismetMathLibrary.MakeTransform` (`self.K2_GetActorLocation`) (`KismetMathLibrary.RandomRotator` false)) "Undefined" "OverrideRootScale" null null)
        (elif (> (`KismetMathLibrary.RandomInteger` 4) 0)
          (`|SpawnActorFromClass` "/Game/kuwano_folder/BP/BP_ItemMoney.BP_ItemMoney_C" (`KismetMathLibrary.MakeTransform` (`self.K2_GetActorLocation`) (`KismetMathLibrary.RandomRotator` false)) "Undefined" "OverrideRootScale" null null))))
    (`self.K2_DestroyActor`)))

(event `self.ReceiveBeginPlay`
  (`parent.ReceiveBeginPlay`)
  (bind _asenemy_hp_blueprint (cast `/Game/kageyama_Folder/enemy/enemy1/enemy_HP_Blueprint` (`WidgetComponent.GetUserWidgetObject` (`self.Widget`))))
  (set `self.Vital Widget` _asenemy_hp_blueprint))

(event `self.ReceiveTick`
  (params (DeltaSeconds :type "Float (single-precision)"))
  (bind _widget (`self.Widget`))
  (bind _vital_widget (`self.Vital Widget`))
  (set `/Game/kageyama_Folder/enemy/enemy1/enemy_HP_Blueprint.Current Value` (`self.HP`) _vital_widget)
  (set `/Game/kageyama_Folder/enemy/enemy1/enemy_HP_Blueprint.Max Value` (`self.Max HP`) _vital_widget)
  (`SceneComponent.K2_SetWorldRotation` (`self.Widget`) (`KismetMathLibrary.FindLookAtRotation` (`SceneComponent.K2_GetComponentLocation` (`self.Widget`)) (`PlayerCameraManager.GetCameraLocation` (`GameplayStatics.GetPlayerCameraManager` 0))) false false)
  (if (<= (`self.GetDistanceTo` (`GameplayStatics.GetPlayerPawn` 0)) 1000.0)
    (`SceneComponent.SetHiddenInGame` _widget false false)
    (else
      (`SceneComponent.SetHiddenInGame` _widget true false))))

(event `self.Box.OnComponentBeginOverlap`
  (params (OverlappedComponent :type "PrimitiveComponent Object Reference") (OtherActor :type "Actor Object Reference") (OtherComp :type "PrimitiveComponent Object Reference") (OtherBodyIndex :type Integer) (bFromSweep :type Boolean) (SweepResult :type "HitResult Structure (by ref)"))
  (if (== OtherActor (`GameplayStatics.GetPlayerCharacter` 0))
    (`/Engine/EditorBlueprintResources/StandardMacros.DoOnce` false :!label _label
      (:`Completed`
        (`GameplayStatics.ApplyDamage` OtherActor (`self.Damage`))
        (`KismetSystemLibrary.Delay` 0.2)
        (goto _label :!via `Reset`)))))

(event `weaponDeacive`
  (`PrimitiveComponent.SetCollisionEnabled` (`self.Box`) "NoCollision"))

(event `WeaponActive`
  (`PrimitiveComponent.SetCollisionProfileName` (`self.Box`) "OverlapAll" true))

(event `Attack`
  (`|PlayMontage` (`self.Mesh`) "/Game/kageyama_Folder/enemy/enemy_anim/zombie_attack_Montage.zombie_attack_Montage"))

(fn `UserConstructionScript`)